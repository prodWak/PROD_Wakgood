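; Base NPC actor that shows a prompt widget near the player and displays line-by-line dialogue.
; Trigger overlaps toggle the widget for any overlapping actor, while actor overlaps with BP_ThirdPersonCharacter call EnterInteraction or ExitInteraction.
; Leaving an interaction also reattaches the character's FollowCamera to its CameraBoom.
; Talk increments an index into the Dialogue array, creates WB_Dialogue as needed, and removes it after the last line.
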(event OnComponentEndOverlap(Trigger)
  (params (OverlappedComponent :type Primitive%20Component%20Object%20Reference) (OtherActor :type Actor%20Object%20Reference) (OtherComp :type Primitive%20Component%20Object%20Reference) (OtherBodyIndex :type Integer))
  ;[1 1 1] Widget Visibility
  (Rendering|SetVisibility (Variables|Default|GetWidget) false false))

(event OnComponentBeginOverlap(Trigger)
  (params (OverlappedComponent :type Primitive%20Component%20Object%20Reference) (OtherActor :type Actor%20Object%20Reference) (OtherComp :type Primitive%20Component%20Object%20Reference) (OtherBodyIndex :type Integer) (bFromSweep :type Boolean) (SweepResult :type Hit%20Result%20Structure%20%28by%20ref%29))
  ;[1 1 1] Widget Visibility
  (Rendering|SetVisibility (Variables|Default|GetWidget) true false))

(event Collision|EventActorEndOverlap
  (params (OtherActor :type Actor%20Object%20Reference))
  ;[1 1 1] Interacting
  (bind _asbp_third_person_character (Utilities|Casting|CastToBP_ThirdPersonCharacter OtherActor))
  (if (Variables|Default|GetisInteracting)
    (Class|BaseNPC|ExitInteraction)
    (bind _returnvalue (Actor|GetActorOfClass "/Game/ThirdPerson/Blueprints/BP_ThirdPersonCharacter.BP_ThirdPersonCharacter_C"))
    (Transformation|AttachComponentToComponent (Variables|/Game/ThirdPerson/Blueprints/BP_ThirdPersonCharacter.BP_ThirdPersonCharacter_C|GetFollowCamera _asbp_third_person_character) (Variables|/Game/ThirdPerson/Blueprints/BP_ThirdPersonCharacter.BP_ThirdPersonCharacter_C|GetCameraBoom _returnvalue) "None" "KeepRelative" "KeepRelative" "KeepRelative" true)))

(event EventTalk
  ;[1 1 1] Talk
  (Math|Integer|IncrementInt (Variables|Default|Gettalkindex)
    (:%20%20
      (if (< (Variables|Default|Gettalkindex) (Utilities|Array|Length (Variables|Default|Getdialogue)))
        (Variables|Default|GetUI
          (:then
            _)
          (:else
            (bind _returnvalue (UserInterface|CreateWidget "/Game/PROD_Wakgood/Dialogue/WB_Dialogue.WB_Dialogue_C" (Game|GetPlayerController 0)))
            (bind _output_get (Variables|Default|SetUI _returnvalue))
            (UserInterface|Viewport|AddtoViewport _output_get 0)))
        (Rendering|Components|TextRender|SetText (Variables|/Game/PROD_Wakgood/Dialogue/WB_Dialogue.WB_Dialogue_C|GetTalktext (Variables|Default|GetUI)) (Utilities|Text|ToText(String) (Utilities|Array|Get(acopy) (Variables|Default|Getdialogue) (Variables|Default|Gettalkindex))))
        (else
          (Widget|RemovefromParent (Variables|Default|GetUI)))))))

(event Collision|EventActorBeginOverlap
  (params (OtherActor :type Actor%20Object%20Reference))
  ;[1 1 1] Interacting
  (Utilities|Casting|CastToBP_ThirdPersonCharacter OtherActor)
  (if (not (Variables|Default|GetisInteracting))
    (Class|BaseNPC|EnterInteraction)))

(fn ConstructionScript)